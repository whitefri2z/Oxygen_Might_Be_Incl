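; BP_Gaz is one cell of a gas simulation, randomly seeded at construction as void or one of four gases with a quantity.
; A looping 0.2s timer updates its Niagara particles and text widget, then checks one neighbour, rotating through four overlap boxes.
; Gas evens out into lower same-type cells and halves into void ones.
; Differing gases swap through type-based rules and random chance, letting hydrogen rise and oxygen rise through carbon dioxide.
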(event Custom|customGameTick
  (bind _nextbox_ (Variables|Default|GetnextBox?))
  (bind _nextbox__2 (Variables|Default|GetnextBox?))
  (if (Utilities|Enum|NotEqual(Enum) (Variables|Default|GetGaz%20Type) "NewEnumerator0")
    (CallFunction|Reconstruct)
    (bind _asbp_gaz (Utilities|Casting|CastToBP_Gaz (Utilities|Array|Get(acopy) (Collision|GetOverlappingActors (Utilities|Select :Index (Variables|Default|GetnextBox?) :Option%200 (Variables|Default|Getup%20box) :Option%201 (Variables|Default|Getleft%20box) :Option%202 (Variables|Default|Getright%20box) :Option%203 (Variables|Default|Getbottom%20box)) "BP_Gaz_C" :!class /Script/Engine.PrimitiveComponent))))
    (Variables|Default|SetTargetGaz _asbp_gaz)
    (if (Utilities|Enum|Equal(Enum) (Variables|BP_Gaz_C|GetGaz%20Type _asbp_gaz) (Variables|Default|GetGaz%20Type))
      (if (> (Variables|Default|GetGaz%20Quantity) (Variables|BP_Gaz_C|GetGaz%20Quantity _asbp_gaz))
        (bind _output_get (Variables|BP_Gaz_C|SetGaz%20Quantity _asbp_gaz (/ (+ (Variables|Default|GetGaz%20Quantity) (Variables|BP_Gaz_C|GetGaz%20Quantity _asbp_gaz)) 2.0)))
        (Variables|Default|SetGaz%20Quantity _output_get))
      (elif (Utilities|Enum|Equal(Enum) (Variables|BP_Gaz_C|GetGaz%20Type _asbp_gaz) "NewEnumerator0")
        (Variables|BP_Gaz_C|SetGaz%20Type _asbp_gaz (Variables|Default|GetGaz%20Type))
        (bind _output_get_2 (Variables|BP_Gaz_C|SetGaz%20Quantity _asbp_gaz (/ (Variables|Default|GetGaz%20Quantity) 2.0)))
        (Variables|Default|SetGaz%20Quantity _output_get_2)
        (else
          (switch Utilities|FlowControl|Switch|SwitchonEnum_GazType (Variables|Default|GetGaz%20Type)
            (:NewEnumerator0
              (Development|PrintString "nani"))
            (:NewEnumerator1
              (if (== _nextbox__2 0)
                (CallFunction|SwitchGazes (Variables|Default|GetTargetGaz))
                (elif (and (!= _nextbox__2 3) (== (Math|Random|RandomIntegerinRange 0 10) 5))
                  (CallFunction|SwitchGazes (Variables|Default|GetTargetGaz)))))
            (:NewEnumerator2
              (if (Utilities|Enum|Equal(Enum) (Variables|BP_Gaz_C|GetGaz%20Type (Variables|Default|GetTargetGaz)) "NewEnumerator4") :!label _label
                (if (== _nextbox_ 0)
                  (CallFunction|SwitchGazes (Variables|Default|GetTargetGaz))
                  (elif (and (!= _nextbox_ 3) (== (Math|Random|RandomIntegerinRange 0 10) 5))
                    (CallFunction|SwitchGazes (Variables|Default|GetTargetGaz))))
                (elif (and (not (Utilities|Enum|Equal(Enum) (Variables|BP_Gaz_C|GetGaz%20Type (Variables|Default|GetTargetGaz)) "NewEnumerator1")) (== (Math|Random|RandomIntegerinRange 0 20) 10))
                  (CallFunction|SwitchGazes (Variables|Default|GetTargetGaz)))))
            (:NewEnumerator3
              (goto _label))))))))

(event Custom|Reconstruct
  ;[0.5284 0.9502 1] End of Each Ticks
  (Effects|Components|ParticleSystem|SetFloatParameter (Variables|Default|GetNiagara) "OxygenQuantity" (Math|Float|SelectFloat 0.0 (Variables|Default|GetGaz%20Quantity) (Utilities|Enum|Equal(Enum) (Variables|Default|GetGaz%20Type) "NewEnumerator0")))
  (Niagara|SetNiagaraVariable(LinearColor) (Variables|Default|GetNiagara) "ParticleColors" (Utilities|Select :Index (Variables|Default|GetGaz%20Type) :NewEnumerator0 "" :NewEnumerator1 (Math|Color|MakeColor 1.0 0.0 0.14) :NewEnumerator2 (Math|Color|MakeColor 0.0 1.0 0.88) :NewEnumerator3 (Math|Color|MakeColor 0.0 1.0 0.27) :NewEnumerator4 (Math|Color|MakeColor 0.07 0.08 0.02)))
  (Variables|Default|SetnextBox? (Math|Integer|%(Integer) (+ (Variables|Default|GetnextBox?) 1) 4))
  (bind _aswbp_gaz (Utilities|Casting|CastToWBP_Gaz (UserInterface|GetWidget (Variables|Default|GetWidget))))
  (Default|ChangeText _aswbp_gaz (Variables|Default|GetGaz%20Quantity) (Variables|Default|GetGaz%20Type)))

(event EventBeginPlay
  (Utilities|Time|SetTimerbyEvent (delegate Custom|customGameTick) 0.2 true))

(fn ConstructionScript
  ;[1 0.3333 0.3333] Randomisation Beam !
  (if (== (Math|Random|RandomIntegerinRange 0 5) 2)
    (Variables|Default|SetGaz%20Type (Utilities|Select :Index (Math|Random|RandomIntegerinRange 0 3) :Option%200 "NewEnumerator1" :Option%201 "NewEnumerator2" :Option%202 "NewEnumerator3" :Option%203 "NewEnumerator4"))
    (Variables|Default|SetGaz%20Quantity (Math|Random|RandomFloatinRange 1e+02 1e+03))
    (else
      (Variables|Default|SetGaz%20Type "NewEnumerator0")))
  ;[1 0.982 0.3033] SetUp Gaz
  (Effects|Components|ParticleSystem|SetFloatParameter (Variables|Default|GetNiagara) "OxygenQuantity" (Math|Float|SelectFloat 0.0 (Variables|Default|GetGaz%20Quantity) (Utilities|Enum|Equal(Enum) (Variables|Default|GetGaz%20Type) "NewEnumerator0")))
  (Niagara|SetNiagaraVariable(LinearColor) (Variables|Default|GetNiagara) "ParticleColors" (Utilities|Select :Index (Variables|Default|GetGaz%20Type) :NewEnumerator0 "" :NewEnumerator1 (Math|Color|MakeColor 1.0 0.0 0.14) :NewEnumerator2 (Math|Color|MakeColor 0.0 1.0 0.88) :NewEnumerator3 (Math|Color|MakeColor 0.0 1.0 0.27) :NewEnumerator4 (Math|Color|MakeColor 0.07 0.08 0.02))))

(fn SwitchGazes
  (params (Target%20for%20Switch :type BP%20Gaz%20Object%20Reference))
  (LocalVariables|Settemp%20Quantity (Variables|BP_Gaz_C|GetGaz%20Quantity Target%20for%20Switch))
  (LocalVariables|Settemp%20Type (Variables|BP_Gaz_C|GetGaz%20Type Target%20for%20Switch))
  (Variables|BP_Gaz_C|SetGaz%20Quantity Target%20for%20Switch (Variables|Default|GetGaz%20Quantity))
  (Variables|BP_Gaz_C|SetGaz%20Type Target%20for%20Switch (Variables|Default|GetGaz%20Type))
  (Variables|Default|SetGaz%20Quantity (LocalVariables|Gettemp%20Quantity))
  (Variables|Default|SetGaz%20Type (LocalVariables|Gettemp%20Type))
  (return))